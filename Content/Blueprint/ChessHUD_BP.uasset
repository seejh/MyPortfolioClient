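; ChessHUD_BP is the chess game's HUD Blueprint, which builds and stores the UI widgets on BeginPlay for player controller 0.
; It adds both players' point displays, a 2D projection widget and a material switching tab to the viewport.
; It also creates the winning screen and replay widget without displaying them, passing the replay widget to the winning screen as its ReplayScreen.
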(event EventBeginPlay
  ;[1 1 1] Adding Player1PointBP to ViewPort
  (bind _returnvalue (UserInterface|CreateWidget "/Game/Blueprint/Player1Point_BP.Player1Point_BP_C" (Game|GetPlayerController 0)))
  (bind _output_get (Variables|Default|SetwidgetPoint1 _returnvalue))
  (UserInterface|Viewport|AddtoViewport _output_get 0)
  ;[1 1 1] Adding Player2PointBP to ViewPort
  (bind _returnvalue_2 (UserInterface|CreateWidget "/Game/Blueprint/Player2Point_BP.Player2Point_BP_C" (Game|GetPlayerController 0)))
  (bind _output_get_2 (Variables|Default|SetwidgetPoint2 _returnvalue_2))
  (UserInterface|Viewport|AddtoViewport _output_get_2 0)
  (Variables|/Script/Chess.ChessPointsWidget|SetPlayerPointTextBlock (Variables|Default|GetwidgetPoint1) (Variables|/Script/Chess.ChessPointsWidget|GetPlayerPointTextBlock (Variables|Default|GetwidgetPoint1)))
  (Variables|/Script/Chess.ChessPointsWidget|SetPlayerPointTextBlock (Variables|Default|GetwidgetPoint2) (Variables|/Script/Chess.ChessPointsWidget|GetPlayerPointTextBlock (Variables|Default|GetwidgetPoint2)))
  ;[1 1 1] Assigning Projection 2D Widget
  (bind _returnvalue_3 (Game|ConstructObjectfromClass "/Game/Blueprint/Projection2D_bP.Projection2D_BP_C" (Game|GetPlayerController 0)))
  (bind _output_get_3 (Variables|Default|Setprojection2DWidget _returnvalue_3))
  (UserInterface|Viewport|AddtoViewport _output_get_3 0)
  ;[1 1 1] Assinging Material Switching Tab
  (bind _returnvalue_4 (Game|ConstructObjectfromClass "/Game/Blueprint/MaterialSwitch.MaterialSwitch_C" (Game|GetPlayerController 0)))
  (bind _output_get_4 (Variables|Default|SetMaterialSwitchingTab _returnvalue_4))
  (UserInterface|Viewport|AddtoViewport _output_get_4 0)
  ;[1 1 1] Assigning Winning Screen
  (bind _returnvalue_5 (UserInterface|CreateWidget "/Game/Blueprint/WinningScreen.WinningScreen_C" (Game|GetPlayerController 0)))
  (Variables|Default|SetwinningScreen _returnvalue_5)
  ;[1 1 1] Assigning Replay Widget
  (bind _returnvalue_6 (UserInterface|CreateWidget "/Game/Blueprint/ReplayChessUserWidgetBP.ReplayChessUserWidgetBP_C" (Game|GetPlayerController 0)))
  (Variables|Default|SetreplayUserWidget _returnvalue_6)
  (Variables|/Script/Chess.WinningScreenWidget|SetReplayScreen (Variables|Default|GetwinningScreen) _returnvalue_6))

(event Collision|EventActorBeginOverlap
  (params (OtherActor :type Actor%20Object%20Reference)))

(event EventTick
  (params (DeltaSeconds :type Float%20%28single-precision%29)))

(fn ConstructionScript)